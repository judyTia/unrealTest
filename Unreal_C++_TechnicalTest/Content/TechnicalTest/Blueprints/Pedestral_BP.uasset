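; Elemental pedestal that holds a pickable on its PickableMagnet and checks whether its element matches the pedestal's own.
; A matching drop, or removal of a match, toggles the particle effect and calls OnStateChanged.
; CanBeManuallyDroppedOn controls the magnet and mesh visibility, while the game mode's elemental definition supplies that mesh's material.
; Helper functions spawn, destroy or re-element the held sphere, or block its pickup.
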(event `self.ReceiveBeginPlay`
  (`self.RefreshMaterial`))

(event `self.PickableMagnet.OnDropEvent`
  (params (pickable :type "PickableComponent Object Reference"))
  (bind _output_get (set `self.bValidElement` (`|EnumEquality` (`ElementalComponent.ElementType` (`self.GetComponentByClass` (`ActorComponent.GetOwner` pickable) "/Script/TechnicalTest.ElementalComponent")) (`ElementalComponent.ElementType` (`self.Elemental`)))))
  (if _output_get
    (`SceneComponent.SetVisibility` (`self.ParticleSystem`) (`self.bValidElement`) false :!label _label)
    (`self.OnStateChanged`)))

(event `self.PickableMagnet.OnPickupEvent`
  (params (pickable :type "PickableComponent Object Reference"))
  (if (`self.bValidElement`)
    (set `self.bValidElement` false)
    (goto _label)))

(fn `DeactivateCurrentPickable`
  (set `PickableComponent.bCanBePickedUp` false (`PickableMagnetComponent.CurrentPickable` (`self.PickableMagnet`))))

(fn `DestroyElementalSphere`
  (bind _pickablemagnet (`self.PickableMagnet`))
  (bind _currentpickable (`PickableMagnetComponent.CurrentPickable` _pickablemagnet))
  (`self.K2_DestroyActor` (`ActorComponent.GetOwner` _currentpickable))
  (`PickableMagnetComponent.DetachPickable` _pickablemagnet _currentpickable))

(fn `RefreshMaterial`
  (bind _asttgame_mode_bp (cast `/Game/TechnicalTest/Blueprints/TTGameMode_BP` (`GameplayStatics.GetGameMode`)))
  (bind _returnvalue (`TTGameMode.GetElementalDefinition` _asttgame_mode_bp (`ElementalComponent.ElementType` (`self.Elemental`))))
  (`PrimitiveComponent.SetMaterial` (`self.StaticMesh1`) 0 (`.Material` (break `ElementalDefinition` _returnvalue))))

(fn `SetElementalSphereElement`
  (params (Element :type Byte))
  (bind _currentpickable (`PickableMagnetComponent.CurrentPickable` (`self.PickableMagnet`)))
  (bind _returnvalue (`self.GetComponentByClass` (`ActorComponent.GetOwner` _currentpickable) "/Script/TechnicalTest.ElementalComponent"))
  (`/Engine/EditorBlueprintResources/StandardMacros.IsValid` _currentpickable
    (:`Is Valid`
      (`/Engine/EditorBlueprintResources/StandardMacros.IsValid` _returnvalue
        (:`Is Valid`
          (`ElementalComponent.SetElement` _returnvalue Element))))))

(fn `SpawnElementalSphere`
  (params (Element :type Byte))
  (bind (_returnvalue_location _returnvalue_rotation) (`KismetMathLibrary.BreakTransform` (`SceneComponent.K2_GetComponentToWorld` (`self.PickableMagnet`))))
  (bind _returnvalue (`|SpawnActorFromClass` "/Game/TechnicalTest/Blueprints/ElementalSphere_BP.ElementalSphere_BP_C" (`KismetMathLibrary.MakeTransform` _returnvalue_location _returnvalue_rotation) "AlwaysSpawn" "OverrideRootScale" null null))
  (`/Game/TechnicalTest/Blueprints/ElementalSphere_BP.SetElement` _returnvalue Element)
  (`PickableMagnetComponent.AttachPickable` (`self.PickableMagnet`) (`self.GetComponentByClass` _returnvalue "/Script/TechnicalTest.PickableComponent")))

(fn `UserConstructionScript`
  (bind _bcanbemanuallydroppedon (`self.bCanBeManuallyDroppedOn`))
  (`SceneComponent.SetVisibility` (`self.StaticMesh1`) _bcanbemanuallydroppedon false)
  (set `PickableMagnetComponent.bActive` _bcanbemanuallydroppedon (`self.PickableMagnet`)))