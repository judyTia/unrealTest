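; Gate actor that swings open once all of its linked pedestals hold a valid element.
; On BeginPlay it binds to each pedestal's state-change event, re-checking every pedestal whenever one fires.
; When all are valid, a timeline rotates the two door pivots apart in yaw, and a flag optionally deactivates each pedestal's current pickable.
; The gate has no closing logic.
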(event `self.ReceiveBeginPlay`
  (for _array_element (`self.LInkedPedestral`)
    (add `/Game/TechnicalTest/Blueprints/Pedestral_BP.OnStateChanged` _array_element (delegate `OnPedestralsStateChanged`))))

(event `OnPedestralsStateChanged`
  (`self.RefreshDoorState`))

(event `Open`
  (bind (_direction _newtrack_0) (`Timeline|Timeline_0`)
    (:`Update`
      (`SceneComponent.K2_SetRelativeRotation` (`self.DoorPivot1`) (`KismetMathLibrary.MakeRotator` 0.0 0.0 (`KismetMathLibrary.Lerp` -180.0 -100.0 _newtrack_0)) false false)
      (`SceneComponent.K2_SetRelativeRotation` (`self.DoorPivot`) (`KismetMathLibrary.MakeRotator` 0.0 0.0 (`KismetMathLibrary.Lerp` 0.0 -80.0 _newtrack_0)) false false))))

(fn `RefreshDoorState`
  (locals (bShouldBeOpen :type Boolean :default true))
  (for _array_element (`self.LInkedPedestral`)
    (bind _output_get (set `local.bShouldBeOpen` (`/Game/TechnicalTest/Blueprints/Pedestral_BP.bValidElement` _array_element)))
    (if (not _output_get)
      (break)))
  (if (`local.bShouldBeOpen`)
    (`self.Open`)
    (if (`self.bDisableLinkedPedestral`)
      (for _array_element_2 (`self.LInkedPedestral`)
        (`/Game/TechnicalTest/Blueprints/Pedestral_BP.DeactivateCurrentPickable` _array_element_2)))))

(fn `UserConstructionScript`)