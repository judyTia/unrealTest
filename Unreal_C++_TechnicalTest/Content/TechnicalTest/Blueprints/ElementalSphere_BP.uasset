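; Elemental sphere actor whose material reflects the element type held by its Elemental component.
; RefreshMaterial casts the game mode to TTGameMode_BP, looks up the definition for the current ElementType and applies its material to the Sphere.
; It runs on construction, BeginPlay and the component's element-changed event.
; SetElement forwards a new element to the component.
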(event `self.ReceiveBeginPlay`
  (`self.RefreshMaterial`))

(event `self.Elemental.OnElementChangedEvent`
  (`self.RefreshMaterial`))

(fn `RefreshMaterial`
  (bind _asttgame_mode_bp (cast `/Game/TechnicalTest/Blueprints/TTGameMode_BP` (`GameplayStatics.GetGameMode`)))
  (bind _returnvalue (`TTGameMode.GetElementalDefinition` _asttgame_mode_bp (`ElementalComponent.ElementType` (`self.Elemental`))))
  (`PrimitiveComponent.SetMaterial` (`self.Sphere`) 0 (`.Material` (break `ElementalDefinition` _returnvalue))))

(fn `SetElement`
  (params (Element :type Byte))
  (`ElementalComponent.SetElement` (`self.Elemental`) Element))

(fn `UserConstructionScript`
  (`self.RefreshMaterial`))